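; BP_MovingEnemy is an enemy that chases the player's TwinStickPawn and can be destroyed by damage.
; When PawnSensing sees a TwinStickPawn, AIMoveTo sends the enemy toward it as the target actor.
; TakeDamage subtracts damage from Health and prints the result while Health is above zero.
; The actor is destroyed only by a further hit after Health has already reached zero or below.
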(event `self.PawnSensing.OnSeePawn`
  (params (Pawn :type "Pawn Object Reference"))
  (bind _astwin_stick_pawn (cast `/Game/TwinStickBP/Blueprints/TwinStickPawn` Pawn))
  (`|AIMoveTo` self (0.0 0.0 0.0) _astwin_stick_pawn))

(event `/Game/BP/BPI_Damageable.TakeDamage`
  (params (Damage :type "Float (single-precision)"))
  (if (> (`self.Health`) 0.0)
    (bind _output_get (set `self.Health` (- (`self.Health`) Damage)))
    (`KismetSystemLibrary.PrintString` (`KismetStringLibrary.Conv_DoubleToString` _output_get) true true (struct :`R` 1.0 :`G` 0.483362 :`A` 1.0))
    (else
      (`self.K2_DestroyActor`))))

(fn `UserConstructionScript`)