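; BP_Enemy is an enemy actor that damages what it overlaps and can be destroyed by incoming damage.
; On overlap it sends a fixed damage message to the other actor, with no check that it is the player.
; Its TakeDamage event subtracts from Health and prints the result while Health is positive.
; Otherwise it calls Die to destroy the actor, so death takes one more hit after Health runs out.
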(event `self.ReceiveActorBeginOverlap`
  (params (OtherActor :type "Actor Object Reference"))
  ;[1 1 1] Do damage to player
  (message `/Game/BP/BPI_Damageable.TakeDamage` OtherActor 20.0))

(event `self.TakeDamage`
  (params (Damage :type "Float (single-precision)"))
  ;[1 1 1] Get Damage from player
  (if (> (`self.Health`) 0.0)
    (bind _output_get (set `self.Health` (- (`self.Health`) Damage)))
    (`KismetSystemLibrary.PrintString` (`KismetStringLibrary.Conv_DoubleToString` _output_get) true true (struct :`R` 1.0 :`B` 0.098743 :`A` 1.0))
    (else
      (`self.Die`))))

(event `self.Die`
  (`self.K2_DestroyActor`))

(fn `UserConstructionScript`)